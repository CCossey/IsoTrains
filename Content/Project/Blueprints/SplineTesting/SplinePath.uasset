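; SplinePath is a spline path Blueprint that exposes Forward and Backward references through two getter functions, apparently linking it to splines in either direction.
; It holds a Spline component and two pointer components, with empty construction, BeginPlay and Tick logic.
; Disconnected debug nodes would move the pointers to the spline's end location, read in local space, and to the world origin.
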(event EventBeginPlay)

(event EventTick
  (params (DeltaSeconds :type Float%20%28single-precision%29)))

(fn ConstructionScript)

(fn GetForwardSpline
  (return (Variables|Default|GetForward)))

(fn GetBackwardSpline
  (return (Variables|Default|GetBackward)))