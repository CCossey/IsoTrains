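; Map tile that lets the player click pairs of its four edge colliders to lay spline paths between them.
; Every second click builds a spline: opposite edges stay straight, while adjacent ones are reordered by index parity and given curve tangents.
; Splines are recorded in a direction-indexed ConnectedDirections table, which lookup functions search for an onward path or the first existing one.
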(event OnClicked(Plane)
  (params (TouchedComponent :type Primitive%20Component%20Object%20Reference) (ButtonPressed :type Key%20Structure))
  (Development|PrintString (Utilities|GetObjectName TouchedComponent)))

(event OnClicked(NorthCollision)
  (params (TouchedComponent :type Primitive%20Component%20Object%20Reference) (ButtonPressed :type Key%20Structure))
  (CallFunction|PickPoint "NewEnumerator0"))

(event OnClicked(SouthCollision)
  (params (TouchedComponent :type Primitive%20Component%20Object%20Reference) (ButtonPressed :type Key%20Structure))
  (CallFunction|PickPoint "NewEnumerator2"))

(event OnClicked(EastCollision)
  (params (TouchedComponent :type Primitive%20Component%20Object%20Reference) (ButtonPressed :type Key%20Structure))
  (CallFunction|PickPoint "NewEnumerator1"))

(event OnClicked(WestCollision)
  (params (TouchedComponent :type Primitive%20Component%20Object%20Reference) (ButtonPressed :type Key%20Structure))
  (CallFunction|PickPoint "NewEnumerator3"))

(fn ConstructionScript)

(fn MakeSpline
  (params (Point%201 :type Direction%20Enum :default "NewEnumerator0") (Point%202 :type Direction%20Enum :default "NewEnumerator0") (IsCurved :type Boolean))
  (bind _returnvalue (Math|Conversions|ToInteger(Byte) Point%202))
  (bind _returnvalue_2 (Math|Conversions|ToInteger(Byte) Point%201))
  (bind _splinepoints (Variables|Default|GetSplinePoints))
  (bind _splinepoints_2 (Variables|Default|GetSplinePoints))
  (bind _output (Utilities|Array|Get(acopy) _splinepoints _returnvalue_2))
  (bind _output_2 (Utilities|Array|Get(acopy) _splinepoints_2 _returnvalue))
  ;[1 1 1] Creating spline
  (bind _returnvalue_3 (AddComponent|AddSplineComponent false))
  (bind _output_get (LocalVariables|SetNewSpline _returnvalue_3))
  (Spline|SetSplinePoints _output_get (Utilities|Array|MakeArray _output _output_2) "Local" true)
  (if IsCurved
    (CallFunction|GenerateCurveTangents (LocalVariables|GetNewSpline) 0 _output)
    (CallFunction|GenerateCurveTangents (LocalVariables|GetNewSpline) 1 _output_2)
    (Spline|UpdateSpline (LocalVariables|GetNewSpline))
    (else
      (Development|PrintString "Spline is not curved")))
  ;[1 1 1] Setting up spline data
  (CallFunction|MakeDirectionConnection Point%201 Point%202 (Utilities|Struct|MakeSplinePathData (LocalVariables|GetNewSpline) (Utilities|Map|MakeMap 0.0 Point%201 (Spline|GetSplineLength (LocalVariables|GetNewSpline)) Point%202) (Variables|Default|GetTileIndex))))

(fn GenerateCurveTangents
  (params (Spline :type Spline%20Component%20Object%20Reference) (PointIndex :type Integer) (point :type Vector))
  (bind (_x _y _z) (Math|Vector|BreakVector point))
  (Spline|SetTangentatSplinePoint Spline PointIndex (Math|Vector|MakeVector (* _x 1.5) (* _y -1.5) _z) "Local" true))

(fn PrepPoints
  (params (First%20Point :type Direction%20Enum :default "NewEnumerator0") (Second%20Point :type Direction%20Enum :default "NewEnumerator0"))
  (LocalVariables|SetPoint%201 First%20Point)
  (bind _output_get (LocalVariables|SetPoint%202 Second%20Point))
  (bind _returnvalue (CallFunction|CurveCheck (LocalVariables|GetPoint%201) _output_get))
  (bind _output_get_2 (LocalVariables|SetIsCurve _returnvalue))
  (if _output_get_2
    ;[0 0.1535 1] Point Switching (if needed)
    (bind (_new_point_1 _new_point_2) (CallFunction|NeedtoSwitchPoints (LocalVariables|GetPoint%201) (LocalVariables|GetPoint%202)))
    (LocalVariables|SetPoint%201 _new_point_1)
    (LocalVariables|SetPoint%202 _new_point_2)
    (CallFunction|MakeSpline (LocalVariables|GetPoint%201) (LocalVariables|GetPoint%202) (LocalVariables|GetIsCurve))
    (else
      (CallFunction|MakeSpline (LocalVariables|GetPoint%201) (LocalVariables|GetPoint%202) (LocalVariables|GetIsCurve)))))

(fn PickPoint
  (params (PointDirection :type Direction%20Enum :default "NewEnumerator0"))
  ;[1 0 0] Debugging
  (Development|PrintString (Utilities|String|Append (Utilities|GetObjectName self) " " (Utilities|String|EnumtoString PointDirection)))
  (if (Variables|Default|GetFirstHit)
    (Variables|Default|SetFirstHit false)
    (Variables|Default|SetFirstHitDirection PointDirection)
    (else
      (Variables|Default|SetFirstHit true)
      (bind _output_get (Variables|Default|SetSecondHitDirection PointDirection))
      ;[1 0 0] Debugging
      (Development|PrintString (Utilities|String|Append (Utilities|String|EnumtoString _output_get) " to " (Utilities|String|EnumtoString (Variables|Default|GetFirstHitDirection))))
      (CallFunction|PrepPoints (Variables|Default|GetFirstHitDirection) (Variables|Default|GetSecondHitDirection)))))

(fn NeedtoSwitchPoints
  (params (First%20Point :type Direction%20Enum :default "NewEnumerator0") (Second%20Point :type Direction%20Enum :default "NewEnumerator0"))
  (LocalVariables|SetPoint%201 First%20Point)
  (bind _output_get (LocalVariables|SetPoint%202 Second%20Point))
  (if (!= (Math|Integer|%(Integer) (Math|Conversions|ToInteger(Byte) _output_get) 2) 0)
    (return (LocalVariables|GetPoint%202) (LocalVariables|GetPoint%201))
    (else
      (return (LocalVariables|GetPoint%201) (LocalVariables|GetPoint%202)))))

(fn CurveCheck
  (params (Point%201 :type Direction%20Enum :default "NewEnumerator0") (Point%202 :type Direction%20Enum :default "NewEnumerator0"))
  (return (!= (Math|Integer|Absolute(Integer) (- (Math|Conversions|ToInteger(Byte) Point%201) (Math|Conversions|ToInteger(Byte) Point%202))) 2)))

(fn MakeDirectionConnection
  (params (Point%201 :type Direction%20Enum :default "NewEnumerator0") (Point%202 :type Direction%20Enum :default "NewEnumerator0") (Spline%20Data :type Spline%20Path%20Data%20Structure))
  (Utilities|Array|SetArrayElem (Utilities|Struct|BreakConnectedDirection (Utilities|Array|Get(acopy) (Variables|Default|GetConnectedDirections) (Math|Conversions|ToInteger(Byte) Point%201))) (Math|Conversions|ToInteger(Byte) Point%202) Spline%20Data)
  (Utilities|Array|SetArrayElem :TargetArray (Utilities|Struct|BreakConnectedDirection (Utilities|Array|Get(acopy) (Variables|Default|GetConnectedDirections) (Math|Conversions|ToInteger(Byte) Point%202))) :Index (Math|Conversions|ToInteger(Byte) Point%201)))

(fn CheckforSplineAhead
  (params (IncommingDirection :type Direction%20Enum :default "NewEnumerator0") (DesiredDirection :type Direction%20Enum :default "NewEnumerator0"))
  (bind _returnvalue (Math|Conversions|ToInteger(Byte) IncommingDirection))
  (Development|PrintString (Utilities|String|Append "Getting available directions from " (Utilities|String|EnumtoString IncommingDirection)))
  ;[1 1 1] Check for available Paths
  (for (_array_element _array_index) (Utilities|Struct|BreakConnectedDirection (Utilities|Array|Get(acopy) (Variables|Default|GetConnectedDirections) _returnvalue))
    (if (!= _array_index _returnvalue)
      (if (!= (.Path (Utilities|Struct|BreakSplinePathData _array_element)) 0)
        (LocalVariables|SetNewPath (.Path (Utilities|Struct|BreakSplinePathData _array_element)))
        (LocalVariables|SetSelectedDirection (Utilities|Enum|ByteToEnumDirection (Math|Conversions|ToByte(Integer) _array_index))))))
  (Development|PrintString (Utilities|String|Append "Going to go " (Utilities|String|EnumtoString (LocalVariables|GetSelectedDirection)))))

(fn GetNearestPath
  (for _array_element (Variables|Default|GetConnectedDirections)
    (for _array_element_2 (Utilities|Struct|BreakConnectedDirection _array_element)
      (if (!= (.Path (Utilities|Struct|BreakSplinePathData _array_element_2)) 0)
        (return _array_element_2)))))