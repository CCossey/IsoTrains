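; TileMap is a map Blueprint that spawns a grid of Tile actors at BeginPlay.
; It splits a hard-coded string of ones and zeros into characters and spawns one indexed tile for each, wrapping rows every Height entries at 100-unit spacing.
; The character values are unused, so only the string length shapes the grid.
; Spawned tiles are stored in Tiles, and CheckIndex bounds-checks indices against that array.
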(event EventBeginPlay
  (Utilities|FlowControl|Sequence
    (:then_0
      (bind _output_get (Variables|Default|SetDataString (Utilities|String|MakeLiteralString "1111000011110000")))
      (Class|KismetStringLibrary|ReplaceInline _output_get "" "" "IgnoreCase"))
    (:then_1
      (bind _output_get_2 (Variables|Default|SetMyData (Utilities|String|GetCharacterArrayfromString _output_get)))
      (for (_ _array_index) _output_get_2
        (if (== (Math|Integer|%(Integer) _array_index (Variables|Default|GetHeight)) 0)
          (Math|Integer|IncrementInt (Variables|Default|GetNext%20Row)
            (:%20%20
              _)))
        (bind _returnvalue (Game|SpawnActorfromClass "/Game/Project/Blueprints/Map/Tile.Tile_C" (Math|Conversions|ToTransform(Vector) (Math|Vector|MakeVector (* (Math|Integer|%(Integer) _array_index (Variables|Default|GetHeight)) 1e+02) (* (Variables|Default|GetNext%20Row) 1e+02) 0.0)) "Undefined" 0 _array_index 0))
        (Utilities|Array|Add (Variables|Default|GetTiles) _returnvalue)))))

(event Collision|EventActorBeginOverlap
  (params (OtherActor :type Actor%20Object%20Reference)))

(event EventTick
  (params (DeltaSeconds :type Float%20%28single-precision%29)))

(fn ConstructionScript)

(fn CheckIndex
  (params (PossibleIndex :type Integer))
  (if (>= PossibleIndex 0)
    (if (< PossibleIndex (Utilities|Array|Length (Variables|Default|GetTiles)))
      (return true)
      (else
        _)))
  (return false))